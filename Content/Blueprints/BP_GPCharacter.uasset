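; BP_GPCharacter is the player character, handling weapon visuals, team joining and menu hooks.
; On BeginPlay it attaches the same weapon mesh to the body and first-person meshes, split by owner visibility, with collision responses ignored.
; Its events use the BP_GPMainMenu game instance to open the in-game menu, pick the team the first player controller joins, or swap the play menu for the HUD and game-only input.
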(event Custom|DestroyPlayMenuChar
  (bind _asbp_gpmain_menu (Utilities|Casting|CastToBP_GPMainMenu (Game|GetGameInstance)))
  (Default|DestroyPlayMenu _asbp_gpmain_menu)
  (Default|ShowHUD _asbp_gpmain_menu)
  (Input|SetInputModeGameOnly)
  (Variables|/Script/Engine.PlayerController|SetbShowMouseCursor (Game|GetPlayerController 0) false))

(event Custom|ChangeColour
  (bind _asbp_gpmain_menu (Utilities|Casting|CastToBP_GPMainMenu (Game|GetGameInstance)))
  (bind _asgpplayer_controller (Utilities|Casting|CastToGPPlayerController (Game|GetPlayerController 0)))
  (if (Variables|/Game/Blueprints/BP_GPMainMenu.BP_GPMainMenu_C|GetTeam _asbp_gpmain_menu)
    (Class|GPPlayerController|JoinTeam0 _asgpplayer_controller)
    (else
      (Class|GPPlayerController|JoinTeam1 _asgpplayer_controller))))

(event EventBeginPlay
  (bind _weaponmeshfirst (Variables|Default|GetWeaponMeshFirst))
  (bind _weaponmesh (Variables|Default|GetWeaponMesh))
  (Components|StaticMesh|SetStaticMesh _weaponmesh "/Game/weapondraft2.weapondraft2")
  (Class|SceneComponent|Attachto _weaponmesh (Variables|Character|GetMesh) "weapon_right" "KeepRelativeOffset" true)
  (Class|PrimitiveComponent|SetOwnerNoSee _weaponmesh true)
  (Components|StaticMesh|SetStaticMesh _weaponmeshfirst "/Game/weapondraft2.weapondraft2")
  (Class|SceneComponent|Attachto _weaponmeshfirst (Variables|Default|GetFirstPersonMesh) "weapon_right" "KeepRelativeOffset" true)
  (Rendering|SetOnlyOwnerSee _weaponmeshfirst true :!class /Script/Engine.PrimitiveComponent)
  (Collision|SetCollisionResponsetoAllChannels (Variables|Default|GetWeaponMeshFirst) "ECR_Ignore")
  (Collision|SetCollisionResponsetoAllChannels (Variables|Default|GetWeaponMesh) "ECR_Ignore"))

(event Input|ActionEvents|InputActionShowInGameMenu
  (:Pressed
    (bind _asbp_gpmain_menu (Utilities|Casting|CastToBP_GPMainMenu (Game|GetGameInstance)))
    (Default|ShowinGameMenu _asbp_gpmain_menu)))

(fn ConstructionScript)