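; Main menu controller that switches between menu screens and handles hosting, finding and joining LAN sessions.
; LeaveCurrentState hides the current state's widget and sets the next state, while Show events lazily create widgets or re-show cached ones.
; Hosting opens the chosen map as a listen server, and searching fills a scroll box with joinable server entries.
; StartOver hides menus, destroys the session when playing, and reloads the menu level.
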(event Custom|DestroyLoading
  ;[1 1 1] Destroy Loading Screen
  (Widget|SetVisibility (Variables|Widgets|GetGPMM_Loading) "Hidden"))

(event Custom|DestroySettings
  ;[1 1 1] Destroy Settings
  (Widget|SetVisibility (Variables|Widgets|GetGPMM_Settings) "Hidden"))

(event Custom|HostGame
  (params (MaxPlayers :type Integer :default 0) (MAP :type String))
  (bind _returnvalue (Game|GetPlayerController 0))
  ;[1 1 1] Host A Game
  (bind _output_get (Variables|Operations|SetMaxConnections MaxPlayers))
  (CallFunction|ShowLoading)
  (|Session _returnvalue _output_get true
    (:OnSuccess
      (Variables|/Script/Engine.PlayerController|SetbShowMouseCursor _returnvalue false)
      (Variables|StateSettings|SetCurrentState (Variables|StateSettings|GetPlayingState))
      (Game|OpenLevel(byName) (Utilities|String|StringToName MAP) true "listen ,game=GPProject.GPGameMode")
      (Input|SetInputModeGameOnly _returnvalue))))

(event Custom|DestroyHost
  ;[1 1 1] Destroy Host
  (Widget|SetVisibility (Variables|Widgets|GetGPMM_Host) "Hidden"))

(event Custom|ShowLoading
  ;[1 1 1] Show Loading Menu
  (Utilities|LeaveCurrentState (Variables|StateSettings|GetLoadingState)
    (:NewState
      (Utilities|IsValid (Variables|Widgets|GetGPMM_Loading)
        (:Is%20Valid
          (Widget|SetVisibility (Variables|Widgets|GetGPMM_Loading) "Visible"))
        (:Is%20Not%20Valid
          (bind _returnvalue (UserInterface|CreateWidget "/Game/GUI/GPMM_Loading.GPMM_Loading_C" (Game|GetPlayerController 0)))
          (bind _output_get (Variables|Widgets|SetGPMM_Loading _returnvalue))
          (UserInterface|Viewport|AddtoViewport _output_get 0))))))

(event Custom|JoinSelected
  (params (Result :type Blueprint%20Session%20Result%20Structure))
  ;[1 1 1] Join Session
  (|JoinSession (Game|GetPlayerController 0) Result
    (:OnSuccess
      (Utilities|LeaveCurrentState (Variables|StateSettings|GetPlayingState)
        (:NewState
          (CallFunction|DestroyBackground)
          (Utilities|SetInputGame))))))

(event Custom|StartOver
  ;[1 1 1] Back To Main Menu
  (CallFunction|DestroyinGameMenu)
  (CallFunction|DestroyHost)
  (CallFunction|DestroyTeams)
  (CallFunction|DestroyLoading)
  (CallFunction|DestroyServerList)
  (if (== (Variables|StateSettings|GetCurrentState) (Variables|StateSettings|GetPlayingState))
    (|DestroySession (Game|GetPlayerController 0)
      (:OnSuccess
        _)))
  (Game|OpenLevel(byName) "GPMainMenu_Level"))

(event Custom|DestroyInGameMenu
  (bind _returnvalue (Game|GetPlayerController 0))
  ;[1 1 1] Destroy In Game Menu
  (Widget|SetVisibility (Variables|Widgets|GetGP_InGameMenu) "Hidden")
  (Input|SetInputModeGameOnly _returnvalue)
  (Variables|/Script/Engine.PlayerController|SetbShowMouseCursor _returnvalue false))

(event Custom|ShowTeams
  ;[1 1 1] Show Teams Menu
  (Utilities|LeaveCurrentState (Variables|StateSettings|GetTeamsState)
    (:NewState
      (Utilities|IsValid (Variables|Widgets|GetGPMM_Teams)
        (:Is%20Valid
          (Widget|SetVisibility (Variables|Widgets|GetGPMM_Teams) "Visible"))
        (:Is%20Not%20Valid
          (bind _returnvalue (UserInterface|CreateWidget "/Game/GUI/GPMM_Teams.GPMM_Teams_C" (Game|GetPlayerController 0)))
          (bind _output_get (Variables|Widgets|SetGPMM_Teams _returnvalue))
          (UserInterface|Viewport|AddtoViewport _output_get 0))))))

(event Custom|DestroyTeams
  ;[1 1 1] Destroy Teams
  (Widget|SetVisibility (Variables|Widgets|GetGPMM_Teams) "Hidden"))

(event Custom|ShowSettings
  ;[1 1 1] Show Settings Menu
  (Utilities|LeaveCurrentState (Variables|StateSettings|GetSettingsState)
    (:NewState
      (Utilities|IsValid (Variables|Widgets|GetGPMM_Settings)
        (:Is%20Valid
          (Widget|SetVisibility (Variables|Widgets|GetGPMM_Settings) "Visible"))
        (:Is%20Not%20Valid
          (bind _returnvalue (UserInterface|CreateWidget "/Game/GUI/GPMM_Settings.GPMM_Settings_C" (Game|GetPlayerController 0)))
          (bind _output_get (Variables|Widgets|SetGPMM_Settings _returnvalue))
          (UserInterface|Viewport|AddtoViewport _output_get 0))))))

(event Custom|ShowBackground
  ;[1 1 1] Show Background Image
  (Utilities|IsCurrentState (Variables|StateSettings|GetStartupState)
    (:True
      (Utilities|IsValid (Variables|Widgets|GetGPMM_Background)
        (:Is%20Valid
          (Widget|SetVisibility (Variables|Widgets|GetGPMM_Background) "Visible"))
        (:Is%20Not%20Valid
          (bind _returnvalue (UserInterface|CreateWidget "/Game/GUI/GPMM_Background.GPMM_Background_C" (Game|GetPlayerController 0)))
          (bind _output_get (Variables|Widgets|SetGPMM_Background _returnvalue))
          (UserInterface|Viewport|AddtoViewport _output_get 0))))))

(event Custom|EndGame
  ;[1 1 1] End Game
  (CallFunction|DestroyMainMenu)
  (CallFunction|DestroyBackground)
  (CallFunction|EndGame))

(event Custom|DestroyBackground
  ;[1 1 1] Destroy Background
  (Widget|SetVisibility (Variables|Widgets|GetGPMM_Background) "Hidden")
  (Variables|/Script/Engine.PlayerController|SetbShowMouseCursor (Game|GetPlayerController 0) false))

(event Custom|StartGame
  (bind _returnvalue (Game|GetPlayerController 0))
  ;[1 1 1] Load Main Menu And Set Current State To Main Menu State
  (Variables|StateSettings|SetCurrentState (Variables|StateSettings|GetStartupState))
  (CallFunction|ShowBackground)
  (CallFunction|ShowMainMenu)
  (Input|SetInputModeUIOnly _returnvalue 0 false)
  (Variables|/Script/Engine.PlayerController|SetbShowMouseCursor _returnvalue true))

(event Custom|JoinGame
  (bind _returnvalue (Game|GetPlayerController 0))
  ;[1 1 1] Get And Show List Of Available Servers
  (Utilities|LeaveCurrentState (Variables|StateSettings|GetServerListState)
    (:NewState
      (Utilities|IsValid (Variables|Widgets|GetGPMM_Join)
        (:Is%20Valid
          (Widget|SetVisibility (Variables|Widgets|GetGPMM_Join) "Visible"))
        (:Is%20Not%20Valid
          (bind _returnvalue_2 (UserInterface|CreateWidget "/Game/GUI/GPMM_Join.GPMM_Join_C" _returnvalue))
          (bind _output_get (Variables|Widgets|SetGPMM_Join _returnvalue_2))
          (UserInterface|Viewport|AddtoViewport _output_get 0)))
      (Default|SetNoneStatusOff _output_get)
      (Default|SetSearchingStatuson _output_get)
      (bind _results (|FindSessions _returnvalue 100 true)
        (:OnSuccess
          (Variables|Default|SetFoundSessions _results)
          (if (== (Utilities|Array|Length _results) 0)
            (Default|SetSearchingStatusOff (Variables|Widgets|GetGPMM_Join) :!label _label)
            (Default|SetNoneStatuson (Variables|Widgets|GetGPMM_Join))
            (else
              (Default|SetSearchingStatusOff (Variables|Widgets|GetGPMM_Join))
              (for _array_element (Variables|Default|GetFoundSessions)
                (bind _returnvalue_3 (UserInterface|CreateWidget "/Game/GUI/GPMM_Join_Entry.GPMM_Join_Entry_C" (Game|GetPlayerController 0)))
                (Utilities|Array|Add (Variables|Default|GetFoundSessionsWidget) _returnvalue_3)
                (Variables|Widgets|SetGPMM_Join_Entry _returnvalue_3)
                (Default|SetName (Variables|Widgets|GetGPMM_Join_Entry) (Utilities|MakeServerString _array_element))
                (Default|SetSearchResult (Variables|Widgets|GetGPMM_Join_Entry) _array_element)
                (Widget|Panel|AddChild (Variables|/Game/GUI/GPMM_Join.GPMM_Join_C|GetScrollBoxServers (Variables|Widgets|GetGPMM_Join)) (Variables|Widgets|GetGPMM_Join_Entry))))))
        (:OnFailure
          (goto _label))))))

(event Custom|RefreshList
  ;[1 1 1] Refresh Server List
  (for _array_element (Variables|Default|GetFoundSessionsWidget)
    (Widget|RemovefromParent _array_element)
    (Utilities|Array|Clear (Variables|Default|GetFoundSessionsWidget))
    (Variables|StateSettings|SetCurrentState 0))
  (Utilities|Array|Clear (Variables|Default|GetFoundSessionsWidget))
  (Variables|StateSettings|SetCurrentState 0))

(event Custom|ShowMainMenu
  (bind _returnvalue (Game|GetPlayerController 0))
  ;[1 1 1] Show Main Menu
  (Utilities|LeaveCurrentState (Variables|StateSettings|GetMainMenuState)
    (:NewState
      (Utilities|IsValid (Variables|Widgets|GetGPMM_Main)
        (:Is%20Valid
          (Widget|SetVisibility (Variables|Widgets|GetGPMM_Main) "Visible"))
        (:Is%20Not%20Valid
          (bind _returnvalue_2 (UserInterface|CreateWidget "/Game/GUI/GPMM_Main.GPMM_Main_C" (Game|GetPlayerController 0)))
          (bind _output_get (Variables|Widgets|SetGPMM_Main _returnvalue_2))
          (UserInterface|Viewport|AddtoViewport _output_get 0)
          (Input|SetInputModeUIOnly _returnvalue 0 true)
          (Variables|/Script/Engine.PlayerController|SetbShowMouseCursor _returnvalue true))))))

(event Custom|DestroyServerList
  ;[1 1 1] Destroy Server List
  (Widget|SetVisibility (Variables|Widgets|GetGPMM_Join) "Hidden"))

(event Custom|DestroyMainMenu
  ;[1 1 1] Destroy Main Menu
  (Widget|SetVisibility (Variables|Widgets|GetGPMM_Main) "Hidden"))

(event Custom|ShowHost
  ;[1 1 1] Show Host Menu
  (Utilities|LeaveCurrentState (Variables|StateSettings|GetHostState)
    (:NewState
      (Utilities|IsValid (Variables|Widgets|GetGPMM_Host)
        (:Is%20Valid
          (Widget|SetVisibility (Variables|Widgets|GetGPMM_Host) "Visible"))
        (:Is%20Not%20Valid
          (bind _returnvalue (UserInterface|CreateWidget "/Game/GUI/GPMM_Host.GPMM_Host_C" (Game|GetPlayerController 0)))
          (bind _output_get (Variables|Widgets|SetGPMM_Host _returnvalue))
          (UserInterface|Viewport|AddtoViewport _output_get 0))))))