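; HUD that draws a full-screen top-down map of the match on the server only, showing two colored corner zones, buildings and players.
; The construction script derives map size and point scale from the viewport, and WorldToMap2 converts world positions to screen by swapping X/Y, offsetting and scaling.
; DrawHUD outlines each GPBuilding with yaw-rotated corner lines.
; Characters appear as team-colored squares whose border turns blue when carrying the flag.
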(event EventBeginPlay)

(event EventActorBeginOverlap
  (params (OtherActor :type Actor%20Object%20Reference)))

(event EventTick
  (params (DeltaSeconds :type Float%20%28single-precision%29)))

(event EventDrawHUD
  (params (SizeX :type Integer) (SizeY :type Integer))
  (bind (_x _y) (Utilities|GetMapOffsetSplit))
  (bind (_mappos _x_pos _y_pos) (Utilities|WorldtoMap2 "1940.000000,3300.000000,1.000000"))
  (bind _mappos_2 (Utilities|WorldtoMap2 "-1940.000000,-3300.000000,1.000000"))
  (bind _playersize (Variables|Constants|GetPlayerSize))
  (bind _playersize_2 (Variables|Constants|GetPlayerSize))
  (bind _mapsizeplusbounds (Variables|Constants|GetMapSizePlusBounds))
  (bind _mapoffsetminusbounds (Variables|Constants|GetMapOffsetMinusBounds))
  (bind _playerborder (Variables|Constants|GetPlayerBorder))
  (bind _mapsize (Variables|Constants|GetMapSize))
  (bind _gameoffsettransposed (Variables|Constants|GetGameOffsetTransposed))
  (bind (_x_2 _y_2) (Math|Vector2D|BreakVector2D _mapoffsetminusbounds))
  (bind (_x_3 _y_3) (Math|Vector2D|BreakVector2D _mapsizeplusbounds))
  (bind _returnvalue (* 2 _playerborder))
  (bind (_x_4 _y_4) (Math|Vector2D|BreakVector2D _mapsize))
  (bind _transposed (CallFunction|Transpose2D _gameoffsettransposed))
  (bind _returnvalue_2 (Math|Conversions|ToVector(Vector2D) _transposed))
  (bind _returnvalue_3 (* _transposed -1.0))
  (bind _returnvalue_4 (- _playersize_2 _returnvalue))
  (bind _returnvalue_5 (Math|Conversions|ToVector(Vector2D) _returnvalue_3))
  (bind _mappos_3 (Utilities|WorldtoMap2 _returnvalue_2))
  (bind _returnvalue_6 (- _mappos_3 _mappos))
  (bind _mappos_4 (Utilities|WorldtoMap2 _returnvalue_5))
  (bind (_x_5 _y_5) (Math|Vector2D|BreakVector2D _returnvalue_6))
  (bind _returnvalue_7 (- _mappos_2 _mappos_4))
  (bind (_x_6 _y_6) (Math|Vector2D|BreakVector2D _returnvalue_7))
  (if (Networking|IsServer)
    (HUD|DrawRect "(R=0.000000,G=0.000000,B=0.000000,A=1.000000)" 0.0 0.0 (Math|Conversions|ToFloat(Integer) SizeX) (Math|Conversions|ToFloat(Integer) SizeY))
    (HUD|DrawRect "(R=0.420000,G=0.318523,B=0.225504,A=1.000000)" _x_2 _y_2 _x_3 _y_3)
    (HUD|DrawRect "(R=0.585000,G=0.443274,B=0.312975,A=1.000000)" _x _y _x_4 _y_4)
    (HUD|DrawRect "(R=1.000000,G=0.000000,B=0.000000,A=1.000000)" _x _y _x_6 _y_6)
    (HUD|DrawRect "(R=0.046600,G=1.000000,B=0.000000,A=1.000000)" _x_pos _y_pos _x_5 _y_5)
    (CallFunction|DrawBuildings)
    (bind _outactors (Actor|GetAllActorsOfClass 0 "/Game/Blueprints/BP_GPCharacter.BP_GPCharacter_C"))
    (for _array_element _outactors
      (bind _asgpplayer_state (Utilities|Casting|CastToGPPlayerState (Variables|/Script/Engine.Controller|GetPlayerState (Pawn|GetController _array_element))))
      (bind _returnvalue_8 (Class|GPPlayerState|GetHasFlag _asgpplayer_state))
      (HUD|DrawRect (select _returnvalue_8 "(R=0.000000,G=0.227268,B=1.000000,A=1.000000)" "(R=0.000000,G=0.000000,B=0.000000,A=1.000000)") (.CornerX (Utilities|PlayerMapGetCorner (.MapPos (Utilities|WorldtoMap2 (Transformation|GetActorLocation _array_element))))) (.CornerY (Utilities|PlayerMapGetCorner (.MapPos (Utilities|WorldtoMap2 (Transformation|GetActorLocation _array_element))))) _playersize _playersize)
      (if (== (Variables|/Script/GPProject.GPPlayerState|GetTeam _asgpplayer_state) 0)
        (HUD|DrawRect "(R=0.000000,G=1.000000,B=0.000000,A=1.000000)" (+ (.CornerX (Utilities|PlayerMapGetCorner (.MapPos (Utilities|WorldtoMap2 (Transformation|GetActorLocation _array_element))))) _playerborder) (+ (.CornerY (Utilities|PlayerMapGetCorner (.MapPos (Utilities|WorldtoMap2 (Transformation|GetActorLocation _array_element))))) _playerborder) _returnvalue_4 _returnvalue_4)
        (else
          (HUD|DrawRect "(R=1.000000,G=0.000000,B=0.000000,A=1.000000)" (+ (.CornerX (Utilities|PlayerMapGetCorner (.MapPos (Utilities|WorldtoMap2 (Transformation|GetActorLocation _array_element))))) _playerborder) (+ (.CornerY (Utilities|PlayerMapGetCorner (.MapPos (Utilities|WorldtoMap2 (Transformation|GetActorLocation _array_element))))) _playerborder) _returnvalue_4 _returnvalue_4))))))

(fn ConstructionScript
  (bind _output_get (Variables|Constants|SetMapSize (Utilities|SizeTakeDoubleBorders (Variables|Constants|GetMapOffset) (Viewport|GetViewportSize))))
  (Variables|Constants|SetMapSizePlusBounds (+ _output_get (Variables|Constants|GetPlayerSize)))
  (Variables|Constants|SetMapOffsetMinusBounds (- (Variables|Constants|GetMapOffset) (/ (Variables|Constants|GetPlayerSize) 2.0)))
  (Variables|Constants|SetPointScale (Math|Conversions|ToVector2D(Vector) (/ (Math|Conversions|ToVector(Vector2D) _output_get 0.0) (Math|Conversions|ToVector(Vector2D) (Variables|Constants|GetGameSizeTransposed) 1.0)))))

(fn Transpose2D
  (params (Pos :type Vector%202D%20Structure))
  (bind (_x _y) (Math|Vector2D|BreakVector2D Pos))
  (return (Math|Vector2D|MakeVector2D _y _x)))

(fn Transpose3DTop
  (params (Pos :type Vector :default "0, 0, 0"))
  (bind (_x _y _z) (Math|Vector|BreakVector Pos))
  (return (Math|Vector|MakeVector _y _x _z)))

(fn WorldtoMap
  (params (World%20Pos :type Vector :default "0, 0, 0"))
  (bind _transposed (CallFunction|Transpose3DTop World%20Pos))
  (bind _gameoffsettransposed (Variables|Constants|GetGameOffsetTransposed))
  (bind _pointscale (Variables|Constants|GetPointScale))
  (bind _mapoffset (Variables|Constants|GetMapOffset))
  (bind _returnvalue (Math|Conversions|ToVector(Vector2D) _gameoffsettransposed))
  (bind _returnvalue_2 (Math|Conversions|ToVector(Vector2D) _pointscale 0.0))
  (bind _returnvalue_3 (Math|Conversions|ToVector(Vector2D) _mapoffset))
  (bind _returnvalue_4 (+ _transposed _returnvalue))
  (bind _returnvalue_5 (* _returnvalue_4 _returnvalue_2))
  (bind _returnvalue_6 (+ _returnvalue_5 _returnvalue_3))
  (bind (_x _y) (Math|Vector|BreakVector _returnvalue_6))
  (return (Math|Conversions|ToVector2D(Vector) _returnvalue_6) _x _y))

(fn DrawBuildings
  (bind _outactors (Actor|GetAllActorsOfClass 0 "/Script/GPProject.GPBuilding"))
  (for _array_element _outactors
    (bind _corners (CallFunction|BuildingtoCorners _array_element))
    (for _index (range 0 3)
      (Class|HUD|DrawLine (.X (Math|Vector2D|BreakVector2D (Utilities|Array|Get(acopy) _corners _index))) (.Y (Math|Vector2D|BreakVector2D (Utilities|Array|Get(acopy) _corners _index))) (.X (Math|Vector2D|BreakVector2D (Utilities|Array|Get(acopy) _corners (Math|Integer|%(Integer) (+ _index 1) 4)))) (.Y (Math|Vector2D|BreakVector2D (Utilities|Array|Get(acopy) _corners (Math|Integer|%(Integer) (+ _index 1) 4)))) "(R=0.938805,G=1.000000,B=0.000000,A=1.000000)"))))

(fn BuildingtoCorners
  (params (Building :type GP%20Building%20Object%20Reference))
  (bind _returnvalue (Transformation|GetActorLocation Building))
  (bind _returnvalue_2 (Transformation|GetActorScale3D Building))
  (bind _returnvalue_3 (Transformation|GetActorRotation Building))
  (bind _buildingmeshsize (Variables|Constants|GetBuildingMeshSize))
  (bind _yaw (Class|KismetMathLibrary|BreakRot _returnvalue_3))
  (bind _returnvalue_4 (* _returnvalue_2 _buildingmeshsize))
  (bind (_mappos _x_pos _y_pos) (Utilities|WorldtoMap2 _returnvalue))
  (bind _returnvalue_5 (/ _returnvalue_4 2.0))
  (bind _returnvalue_6 (* _returnvalue_5 "-1.000000,1.000000, 0"))
  (bind _returnvalue_7 (* _returnvalue_5 "1.000000,-1.000000, 0"))
  (bind _returnvalue_8 (* _returnvalue_5 "-1.000000,-1.000000, 0"))
  (bind _returnvalue_9 (+ _returnvalue _returnvalue_5))
  (bind _returnvalue_10 (+ _returnvalue _returnvalue_6))
  (bind _returnvalue_11 (+ _returnvalue _returnvalue_8))
  (bind _returnvalue_12 (+ _returnvalue _returnvalue_7))
  (bind (_mappos_2 _x_pos_2 _y_pos_2) (Utilities|WorldtoMap2 _returnvalue_9))
  (bind (_mappos_3 _x_pos_3 _y_pos_3) (Utilities|WorldtoMap2 _returnvalue_10))
  (bind (_mappos_4 _x_pos_4 _y_pos_4) (Utilities|WorldtoMap2 _returnvalue_11))
  (bind (_mappos_5 _x_pos_5 _y_pos_5) (Utilities|WorldtoMap2 _returnvalue_12))
  (return (Utilities|Array|MakeArray (Utilities|RotateCorner _x_pos _y_pos _yaw _x_pos_2 _y_pos_2) (Utilities|RotateCorner _x_pos _y_pos _yaw _x_pos_5 _y_pos_5) (Utilities|RotateCorner _x_pos _y_pos _yaw _x_pos_4 _y_pos_4) (Utilities|RotateCorner _x_pos _y_pos _yaw _x_pos_3 _y_pos_3))))